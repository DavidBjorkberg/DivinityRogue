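; Actor that draws a movement path from the game mode's in-play character to the location under the cursor.
; DrawMovementSpline clears the previous path, runs a synchronous navigation query, and builds a clamped-curve spline from the path points.
; It adds a shadowless, collision-free spline mesh per segment, matched to the spline's tangents.
; ClearSpline destroys those runtime-created meshes and the spline.
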(event EventClearSpline
  (bind _splinemeshcomponents (Variables|Default|GetSplineMeshComponents))
  (bind _splinecomponent (Variables|Default|GetSplineComponent))
  (Utilities|FlowControl|Sequence
    (:then_0
      (for _array_element _splinemeshcomponents
        (Utilities|IsValid _array_element
          (:Is%20Valid
            (Components|DestroyComponent _array_element))))
      (Utilities|Array|Clear _splinemeshcomponents))
    (:then_1
      (Utilities|IsValid _splinecomponent
        (:Is%20Valid
          (Components|DestroyComponent _splinecomponent))))))

(event EventDrawMovementSpline
  (Utilities|FlowControl|Sequence
    (:then_0
      (Class|DRMovementSpline|ClearSpline))
    (:then_1
      (bind _returnvalue (Class|DRGameplayStatics|GetHitResultUnderCursor "ECC_WorldStatic"))
      (bind _asdrgame_mode (Utilities|Casting|CastToDRGameMode (Game|GetGameMode)))
      (bind _returnvalue_2 (Class|NavigationSystemV1|FindPathtoLocationSynchronously (Transformation|GetActorLocation (Variables|/Script/DivinityRogue.DRGameMode|GetmCharacterInPlay _asdrgame_mode)) (.location _returnvalue) 0 0))
      (bind _returnvalue_3 (AddComponent|AddSplineComponent false))
      (bind _output_get (Variables|Default|SetSplineComponent _returnvalue_3))
      (Spline|SetSplinePoints _returnvalue_3 (Variables|/Script/NavigationSystem.NavigationPath|GetPathPoints _returnvalue_2) "World" true)
      (for _index (range 0 (- (Spline|GetNumberOfSplinePoints _returnvalue_3) 1))
        (Spline|SetSplinePointType _output_get _index "CurveClamped" true))
      (for _index_2 (range 0 (- (Spline|GetNumberOfSplinePoints _returnvalue_3) 2))
        (bind _returnvalue_4 (AddComponent|AddSplineMeshComponent false))
        (Rendering|SetCastShadow _returnvalue_4 false)
        (Collision|SetCollisionEnabled _returnvalue_4 "NoCollision")
        (Utilities|Array|Add (Variables|Default|GetSplineMeshComponents) _returnvalue_4)
        (SplineMesh|SetStartandEnd _returnvalue_4 (.Location (Spline|GetLocationandTangentatSplinePoint _returnvalue_3 _index_2 "Local")) (.Tangent (Spline|GetLocationandTangentatSplinePoint _returnvalue_3 _index_2 "Local")) (.Location (Spline|GetLocationandTangentatSplinePoint _returnvalue_3 (+ _index_2 1) "Local")) (.Tangent (Spline|GetLocationandTangentatSplinePoint _returnvalue_3 (+ _index_2 1) "Local")) true :!class /Script/Engine.SplineMeshComponent)))))

(fn ConstructionScript)