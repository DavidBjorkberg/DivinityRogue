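; Movement path preview actor that draws a spline from the round system's character in play to the ability target under the cursor, or to the cursor's world hit point.
; DrawMovementSpline clears the previous spline, runs a synchronous navigation path query and lifts the points slightly to build a curved spline.
; It then creates one spline mesh per segment at runtime, tracked in an array so ClearSpline can destroy them.
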(event EventClearSpline
  (bind _splinemeshcomponents (Variables|Default|GetSplineMeshComponents))
  (bind _splinecomponent (Variables|Default|GetSplineComponent))
  ;[1 1 1] Clear Spline
  (Utilities|FlowControl|Sequence
    (:then_0
      (for _array_element _splinemeshcomponents
        (Utilities|IsValid _array_element
          (:Is%20Valid
            (Components|DestroyComponent _array_element))))
      (Utilities|Array|Clear _splinemeshcomponents))
    (:then_1
      (Utilities|IsValid _splinecomponent
        (:Is%20Valid
          (Components|DestroyComponent _splinecomponent))))))

(event EventDrawMovementSpline
  (Utilities|FlowControl|Sequence
    (:then_0
      (Class|DRMovementSpline|ClearSpline))
    (:then_1
      (Variables|Default|SetStartPos (Transformation|GetActorLocation (Variables|/Script/DivinityRogue.DRRoundSystem|GetmCharacterInPlay (Class|DRGameplayStatics|GetRoundSystem))))
      (bind _asdrplayer_controller_bp (Utilities|Casting|CastToDRPlayerController_BP (Game|GetPlayerController 0)))
      (Utilities|IsValid (Class|DRPlayerController|GetAbilityTargetUnderCursor _asdrplayer_controller_bp)
        (:Is%20Valid
          (Variables|Default|SetEndPos (Transformation|GetActorLocation (Components|GetOwner (Class|DRPlayerController|GetAbilityTargetUnderCursor _asdrplayer_controller_bp)))))
        (:Is%20Not%20Valid
          (bind _returnvalue (Class|DRGameplayStatics|GetHitResultUnderCursor "ECC_WorldStatic"))
          (Variables|Default|SetEndPos (.location _returnvalue)))))
    (:then_2
      (bind _returnvalue_2 (Class|NavigationSystemV1|FindPathtoLocationSynchronously (Variables|Default|GetStartPos) (Variables|Default|GetEndPos) 0 0))
      (bind _returnvalue_3 (AddComponent|AddSplineComponent false))
      (Variables|Default|SetSplineComponent _returnvalue_3)
      (for (_array_element _array_index) (Variables|/Script/NavigationSystem.NavigationPath|GetPathPoints _returnvalue_2)
        (Utilities|Array|SetArrayElem (Variables|/Script/NavigationSystem.NavigationPath|GetPathPoints _returnvalue_2) _array_index (+ _array_element "0.000000,0.000000,30.000000")))
      (Spline|SetSplinePoints (Variables|Default|GetSplineComponent) (Variables|/Script/NavigationSystem.NavigationPath|GetPathPoints _returnvalue_2) "World" true)
      (for _index (range 0 (- (Spline|GetNumberOfSplinePoints (Variables|Default|GetSplineComponent)) 1))
        (Spline|SetSplinePointType (Variables|Default|GetSplineComponent) _index "Curve" true))
      (for _index_2 (range 0 (- (Spline|GetNumberOfSplinePoints (Variables|Default|GetSplineComponent)) 2))
        (bind _returnvalue_4 (AddComponent|AddSplineMeshComponent false))
        (Utilities|Array|Add (Variables|Default|GetSplineMeshComponents) _returnvalue_4)
        (SplineMesh|SetStartandEnd _returnvalue_4 (.Location (Spline|GetLocationandTangentatSplinePoint (Variables|Default|GetSplineComponent) _index_2 "Local")) (.Tangent (Spline|GetLocationandTangentatSplinePoint (Variables|Default|GetSplineComponent) _index_2 "Local")) (.Location (Spline|GetLocationandTangentatSplinePoint (Variables|Default|GetSplineComponent) (+ _index_2 1) "Local")) (.Tangent (Spline|GetLocationandTangentatSplinePoint (Variables|Default|GetSplineComponent) (+ _index_2 1) "Local")) true :!class /Script/Engine.SplineMeshComponent)))))

(fn ConstructionScript)