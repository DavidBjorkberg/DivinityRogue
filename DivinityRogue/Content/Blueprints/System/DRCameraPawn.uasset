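; Camera pawn for a turn-based game that centers on the active character and otherwise allows free panning.
; On each game-mode new-turn event it jumps to the new character with an XY offset, keeping its own height, and tracks it during the WalkingPath state.
; Outside that state, Tick applies movement input for panning, while the Zoom axis adjusts clamped spring-arm length.
; Screen-edge mouse panning exists but is disabled.
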(event Custom|OnNewTurn
  (params (previousCharacter :type DR%20Character%20Object%20Reference) (newCharacter :type DR%20Character%20Object%20Reference))
  (Variables|Default|SetCurrentCharacter newCharacter)
  (CallFunction|FollowCurrentCharacter))

(event Custom|FollowCurrentCharacter
  (bind _pantonewunitoffset (Variables|Default|GetPanToNewUnitOffset))
  (bind _currentcharacter (Variables|Default|GetCurrentCharacter))
  (bind _returnvalue (Transformation|GetActorLocation _currentcharacter))
  (Utilities|IsValid (Variables|Default|GetCurrentCharacter)
    (:Is%20Valid
      (Transformation|SetActorLocation (Math|Vector|MakeVector (+ (.x _returnvalue) (.x _pantonewunitoffset)) (+ (.y _returnvalue) (.y _pantonewunitoffset)) (.z (Transformation|GetActorLocation))) false false))))

(event EventBeginPlay
  (EventDispatchers|BindEventtoMonNewTurn (Class|DRGameplayStatics|GetDRGameMode) (delegate Custom|OnNewTurn)))

(event EventTick
  (params (DeltaSeconds :type Float%20%28single-precision%29))
  (if (Class|DRGameMode|IsinGameplayState (Class|DRGameplayStatics|GetDRGameMode) "WalkingPath")
    (CallFunction|FollowCurrentCharacter)
    (else
      (Utilities|FlowControl|Sequence
        (:then_0
          (Pawn|Input|AddMovementInput (Math|Vector|MakeVector (Input|AxisValues|GetMoveCameraForward) (Input|AxisValues|GetMoveCameraRight) 0.0) 1.0 false))))))

(event Input|AxisEvents|InputAxisZoom
  (params (AxisValue :type Float%20%28single-precision%29))
  (bind _springarm (Variables|Default|GetSpringArm))
  (Variables|/Script/Engine.SpringArmComponent|SetTargetArmLength _springarm (Math|Float|Clamp(Float) (+ (* (* AxisValue -1.0) (* (Utilities|Time|GetWorldDeltaSeconds) (Variables|Default|GetZoomSpeed))) (Variables|/Script/Engine.SpringArmComponent|GetTargetArmLength _springarm)) (Variables|Default|GetMinCameraDistance) (Variables|Default|GetMaxCameraDistance))))

(fn ConstructionScript)

(fn MouseMoveonAxis
  (params (PositionOnAxis :type Float%20%28double-precision%29) (AxisLength :type Float%20%28double-precision%29) (Axis :type Vector))
  (bind _returnvalue (- AxisLength PositionOnAxis))
  (if (< _returnvalue 1.0)
    (Pawn|Input|AddMovementInput Axis 1.0 false)
    (elif (> _returnvalue (- AxisLength 1.0))
      (Pawn|Input|AddMovementInput Axis 1.0 false))))