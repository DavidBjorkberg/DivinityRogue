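; DRCameraPawn is a player-controlled camera pawn that pans across the world and zooms on a spring arm.
; Each tick, the MoveCameraForward and MoveCameraRight values drive movement input along world X and Y.
; The Zoom axis adjusts arm length, scaled by speed and delta time and clamped between minimum and maximum distances.
; Screen-edge mouse panning through MouseMoveOnAxis is present but disabled, and pushes the same direction at both edges.
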(event EventTick
  (params (DeltaSeconds :type Float%20%28single-precision%29))
  (Utilities|FlowControl|Sequence
    (:then_0
      (Pawn|Input|AddMovementInput (Math|Vector|MakeVector (Input|AxisValues|GetMoveCameraForward) (Input|AxisValues|GetMoveCameraRight) 0.0) 1.0 false))))

(event Input|AxisEvents|InputAxisZoom
  (params (AxisValue :type Float%20%28single-precision%29))
  (bind _springarm (Variables|Default|GetSpringArm))
  (Variables|/Script/Engine.SpringArmComponent|SetTargetArmLength _springarm (Math|Float|Clamp(Float) (+ (* (* AxisValue -1.0) (* (Utilities|Time|GetWorldDeltaSeconds) (Variables|Default|GetZoomSpeed))) (Variables|/Script/Engine.SpringArmComponent|GetTargetArmLength _springarm)) (Variables|Default|GetMinCameraDistance) (Variables|Default|GetMaxCameraDistance))))

(fn ConstructionScript)

(fn MouseMoveonAxis
  (params (PositionOnAxis :type Float%20%28double-precision%29) (AxisLength :type Float%20%28double-precision%29) (Axis :type Vector))
  (bind _returnvalue (- AxisLength PositionOnAxis))
  (if (< _returnvalue 1.0)
    (Pawn|Input|AddMovementInput Axis 1.0 false)
    (elif (> _returnvalue (- AxisLength 1.0))
      (Pawn|Input|AddMovementInput Axis 1.0 false))))