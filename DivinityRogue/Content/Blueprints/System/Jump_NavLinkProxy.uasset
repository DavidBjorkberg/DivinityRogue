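; Nav link proxy that makes a DRCharacter jump to the link's destination when it reaches the smart link.
; Jump duration depends on team: enemies divide JumpDuration by four times their template's movement speed factor, while others use that factor directly as the duration.
; CalculateVelocity solves a ballistic launch velocity for that duration using hardcoded gravity, and LaunchCharacter applies it, overriding existing velocity.
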(event EventSmartLinkReached
  (params (Agent :type Actor%20Object%20Reference) (Destination :type Vector%20%28by%20ref%29 :default "0, 0, 0"))
  (bind _asdrcharacter (Utilities|Casting|CastToDRCharacter Agent))
  (Utilities|FlowControl|Sequence
    (:then_0
      (if (Utilities|Enum|Equal(Enum) (Class|DRAbilityTargetComponent|GetTeam (Variables|/Script/DivinityRogue.DRCharacter|GetmAbilityTargetComponent _asdrcharacter)) "ENEMY")
        (Variables|Default|SetModifiedJumpDuration (/ (Variables|Default|GetJumpDuration) (* (Variables|/Script/DivinityRogue.DRCharacterTemplate|GetMovementSpeedFactor (Variables|/Script/DivinityRogue.DRCharacter|GetmCharacterTemplate _asdrcharacter)) 4.0)))
        (else
          (Variables|Default|SetModifiedJumpDuration (Variables|/Script/DivinityRogue.DRCharacterTemplate|GetMovementSpeedFactor (Variables|/Script/DivinityRogue.DRCharacter|GetmCharacterTemplate _asdrcharacter))))))
    (:then_1
      (bind _velocity (CallFunction|CalculateVelocity Destination (Transformation|GetActorLocation Agent) (Variables|Default|GetModifiedJumpDuration)))
      (Character|LaunchCharacter _asdrcharacter _velocity true true))))

(fn ConstructionScript)

(fn CalculateVelocity
  (params (DestinationLocation :type Vector) (StartingLocation :type Vector) (Duration :type Float%20%28double-precision%29))
  (bind (_x _y _z) (Math|Vector|BreakVector DestinationLocation))
  (bind (_x_2 _y_2 _z_2) (Math|Vector|BreakVector StartingLocation))
  (LocalVariables|SetInDuration Duration)
  (return (Math|Vector|MakeVector (/ (- _x _x_2) (LocalVariables|GetInDuration)) (/ (- _y _y_2) (LocalVariables|GetInDuration)) (/ (- _z (+ _z_2 (* (Math|Float|Square (LocalVariables|GetInDuration)) -0.5 982.0))) (LocalVariables|GetInDuration)))))