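; DREnemySpawner_BP is a round-based enemy spawner placed in the level.
; It listens to the game mode's new-round event and decrements a countdown shown on a text render component.
; When the countdown reaches zero it resets and asks the game mode to spawn a random character from its enemy list at the spawn point.
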(event Custom|OnNewRound
  (bind _result (Math|Integer|DecrementInt (Variables|Default|GetSpawnTimer))
    (:%20%20
      (if (== _result 0)
        (CallFunction|ResetTimer)
        (CallFunction|SpawnEnemies))
      (CallFunction|UpdateText))))

(event Custom|ResetTimer
  (Variables|Default|SetSpawnTimer (Variables|Default|GetSpawnTime)))

(event Custom|SpawnEnemies
  (Class|DRGameMode|SpawnCharacter (Class|DRGameplayStatics|GetDRGameMode) (.OutItem (Utilities|Array|Random (Variables|Default|GetEnemiesToSpawn))) (Transformation|GetWorldLocation (Variables|Default|GetSpawnPoint))))

(event Custom|UpdateText
  (Rendering|Components|TextRender|SetText (Variables|Default|GetTextRender) (Utilities|Text|ToText(Integer) (Variables|Default|GetSpawnTimer))))

(event EventBeginPlay
  (CallFunction|ResetTimer)
  (EventDispatchers|BindEventtoMonNewRound (Class|DRGameplayStatics|GetDRGameMode) (delegate Custom|OnNewRound)))

(fn ConstructionScript)